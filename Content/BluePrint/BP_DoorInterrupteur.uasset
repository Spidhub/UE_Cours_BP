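; BP_DoorInterrupteur is a switch trigger that activates a set of controllable actors when the third-person character overlaps its collision.
; It stays inert until a dispatcher fires its ActivateControlables event, then sets itself activable and unbinds all listeners from that event.
; Each overlap then calls ActivateMessage on every element of BPControllables that implements the BPI_InterrupteurControl interface.
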(event OnComponentBeginOverlap(Collision)
  (params (OverlappedComponent :type Primitive%20Component%20Object%20Reference) (OtherActor :type Actor%20Object%20Reference) (OtherComp :type Primitive%20Component%20Object%20Reference) (OtherBodyIndex :type Integer) (bFromSweep :type Boolean) (SweepResult :type Hit%20Result%20Structure%20%28by%20ref%29))
  (if (Variables|Default|GetActivable?)
    (Utilities|Casting|CastToBP_ThirdPersonCharacter OtherActor)
    (for _array_element (Variables|Default|GetBP_Controllables)
      (if (Utilities|DoesObjectImplementInterface _array_element "/Game/BluePrint/BPI_InterrupteurControl.BPI_InterrupteurControl_C")
        (Class|BPIInterrupteurControl|Activate(Message) _array_element)))))

(event Custom|Activate
  (Variables|Default|SetActivable? true)
  (EventDispatchers|UnbindallEventsfromActivateControlables (Variables|Default|GetBP_Dispatcher)))

(event EventBeginPlay
  (EventDispatchers|BindEventtoActivateControlables (Variables|Default|GetBP_Dispatcher) (delegate Custom|Activate)))

(fn ConstructionScript)