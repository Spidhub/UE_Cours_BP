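; A door Blueprint that swings open or closed when a referenced dispatcher signals it.
; On BeginPlay it binds its Activate event to the ActivateControlables event dispatcher on BPDispatcher, and Activate calls ToggleDoor.
; ToggleDoor checks the Open flag to run OpenDoor or CloseDoor, each updating the flag and playing its own timeline from the start to drive the door's relative yaw.
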(event Custom|OpenDoor
  (Variables|Default|SetOpen? true)
  (bind _opendoor (Timeline|Opening PlayFromStart)
    (:Update
      (Transformation|SetRelativeRotation (Variables|Default|GetDoor) (Math|Rotator|MakeRotator 0.0 0.0 _opendoor) false false))))

(event Custom|CloseDoor
  (Variables|Default|SetOpen? false)
  (bind _newtrack_0 (Timeline|Closing PlayFromStart)
    (:Update
      (Transformation|SetRelativeRotation (Variables|Default|GetDoor) (Math|Rotator|MakeRotator 0.0 0.0 _newtrack_0) false false))))

(event Custom|ToggleDoor
  (if (Variables|Default|GetOpen?)
    (CallFunction|CloseDoor)
    (else
      (CallFunction|OpenDoor))))

(event Custom|Activate
  (CallFunction|ToggleDoor))

(event EventBeginPlay
  (EventDispatchers|BindEventtoActivateControlables (Variables|Default|GetBP_dispatcher) (delegate Custom|Activate)))

(fn ConstructionScript)