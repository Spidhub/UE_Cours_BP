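; Door actor that swings open or closed when triggered through its Activate and Desactivate interface events, both of which simply toggle it.
; ToggleDoor checks the Open flag, increments or decrements a door count on BPLamp, then calls OpenDoor or CloseDoor.
; Separate Opening and Closing timelines drive the door's relative yaw.
; Both restart from the beginning, so rapid toggling makes the animation jump.
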(event Custom|OpenDoor
  ;[1 1 1] Event lié a ouverture et fermeture des porte avec Timeline (en cas de spam du bouton l'animation n'est pas smooth voir un peu glitché)
  (Variables|Default|SetOpen? true)
  (bind _opendoor (Timeline|Opening PlayFromStart)
    (:Update
      (Transformation|SetRelativeRotation (Variables|Default|GetDoor) (Math|Rotator|MakeRotator 0.0 0.0 _opendoor) false false))))

(event Custom|CloseDoor
  ;[1 1 1] Event lié a ouverture et fermeture des porte avec Timeline (en cas de spam du bouton l'animation n'est pas smooth voir un peu glitché)
  (Variables|Default|SetOpen? false)
  (bind _newtrack_0 (Timeline|Closing PlayFromStart)
    (:Update
      (Transformation|SetRelativeRotation (Variables|Default|GetDoor) (Math|Rotator|MakeRotator 0.0 0.0 _newtrack_0) false false))))

(event Custom|ToggleDoor
  (bind _bp_lamp (Variables|Default|GetBP_Lamp))
  ;[1 1 1] Event actionnant l'ouverture ou la fermeture des portes en fonction de leur états
  (if (Variables|Default|GetOpen?)
    ;;[1 1 1] Communiquer avec Lamp
    (Default|DecrDoor _bp_lamp)
    (CallFunction|CloseDoor)
    (else
      (Default|IncrDoor _bp_lamp)
      (CallFunction|OpenDoor))))

(event EventActivate
  ;[1 1 1] Event de l'interface
  (CallFunction|ToggleDoor))

(event EventDesactivate
  ;[1 1 1] Event de l'interface
  (CallFunction|ToggleDoor))

(fn ConstructionScript)